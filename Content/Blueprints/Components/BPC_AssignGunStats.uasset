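; Actor component that initializes a gun's stats from the DT_GunStats data table.
; On BeginPlay it gets the row name from the owner through GetNameMessage and looks up that row.
; If found, it copies firing, damage, recoil, reload and magazine values onto the owner.
; It also fills the current magazine and sets current ammo to magazine size times max magazines.
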(event EventBeginPlay
  (bind _owner (Variables|Default|GetOwner))
  (bind _name (Class|BPIGuns|GetName(Message) _owner))
  (bind _returnvalue (Utilities|GetDataTableRow "/Game/Blueprints/DataTables/DT_GunStats.DT_GunStats" _name)
    (:then
      (Variables|/Game/Blueprints/Guns/BP_GunParent.BP_GunParent_C|SetIsHitscan _owner (.ishitscan _returnvalue))
      (Variables|/Game/Blueprints/Guns/BP_GunParent.BP_GunParent_C|SetDamage _owner (.damage _returnvalue))
      (Variables|/Game/Blueprints/Guns/BP_GunParent.BP_GunParent_C|SetFirerate _owner (.firerate _returnvalue))
      (Variables|/Game/Blueprints/Guns/BP_GunParent.BP_GunParent_C|SetSpread _owner (.spread _returnvalue))
      (Variables|/Game/Blueprints/Guns/BP_GunParent.BP_GunParent_C|SetRecoil _owner (.recoil _returnvalue))
      (Variables|/Game/Blueprints/Guns/BP_GunParent.BP_GunParent_C|SetReload%20Time _owner (.reloadtime _returnvalue))
      (Variables|/Game/Blueprints/Guns/BP_GunParent.BP_GunParent_C|SetMag%20Size _owner (.magazinesize _returnvalue))
      (Variables|/Game/Blueprints/Guns/BP_GunParent.BP_GunParent_C|SetCurrMagAmmo _owner (.magazinesize _returnvalue))
      (Variables|/Game/Blueprints/Guns/BP_GunParent.BP_GunParent_C|SetMax%20Mags _owner (.maxmagazines _returnvalue))
      (Variables|/Game/Blueprints/Guns/BP_GunParent.BP_GunParent_C|SetCurrAmmo _owner (* (.magazinesize _returnvalue) (.maxmagazines _returnvalue))))))

(event EventTick
  (params (DeltaSeconds :type Float%20%28single-precision%29)))