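; BPC_WeaponSway is a player character component that sways the weapon in response to mouse movement and character velocity.
; On BeginPlay it caches the character, controller and the Arrow1 component's base relative transform.
; Each Tick, unless the character is knifing, a vector spring blends mouse delta with local lateral and vertical velocity, then offsets Arrow1's location opposite to the result.
; Rotation nodes are left unconnected, so only location sways.
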(event EventBeginPlay
  (bind _asbp_player_character (Utilities|Casting|CastToBP_PlayerCharacter (Components|GetOwner)))
  (bind _output_get (Variables|Default|Setcharacter _asbp_player_character))
  (Variables|Default|Setcontroller (Game|GetPlayerController (Variables|/Script/Engine.Pawn|GetPlayerState _output_get)))
  (bind _output_get_2 (Variables|Default|SetweaponBase (Variables|/Game/Blueprints/Player/BP_PlayerCharacter.BP_PlayerCharacter_C|GetArrow1 _output_get)))
  (Variables|Default|SetbaseLocation (Variables|/Script/Engine.SceneComponent|GetRelativeLocation _output_get_2))
  (Variables|Default|SetbaseRotation (Variables|/Script/Engine.SceneComponent|GetRelativeRotation _output_get_2)))

(event EventTick
  (params (DeltaSeconds :type Float%20%28single-precision%29))
  (bind _character (Variables|Default|Getcharacter))
  (bind _controller (Variables|Default|Getcontroller))
  (bind (_deltax _deltay) (Class|PlayerController|GetInputMouseDelta _controller))
  (if (not (Variables|/Game/Blueprints/Player/BP_PlayerCharacter.BP_PlayerCharacter_C|GetKnifing (Variables|Default|Getcharacter)))
    (bind _returnvalue (Class|KismetMathLibrary|VectorSpringInterp (Variables|Default|GetmouseSwayVector) (Math|Vector|MakeVector 0.0 (+ _deltax (/ (.y (Math|Vector|UnrotateVector (Transformation|GetVelocity _character) (Transformation|GetActorRotation _character))) 4e+02)) (+ _deltay (/ (.z (Transformation|GetVelocity (Variables|Default|Getcharacter))) 4e+01))) (Variables|Default|GetswaySpringState) 0.9 0.7 DeltaSeconds 0.006 1.0))
    (bind _output_get (Variables|Default|SetmouseSwayVector _returnvalue))
    (Transformation|SetRelativeLocation (Variables|Default|GetweaponBase) (+ (/ (* _output_get -1) 1.5) (Variables|Default|GetbaseLocation)) false false)))