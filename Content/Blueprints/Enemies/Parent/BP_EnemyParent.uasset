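; Parent enemy character that gets a stats-assignment component and chases the player, reissuing AIMoveTo every Tick unless knocked back.
; Damage awards points to its causer, with a bonus on kills, including bleed and acid kills.
; Bleed and acid use looping timers for stacking damage, refreshing duration on reapplication.
; Knockback launches it with friction briefly removed, while lightning buildup only prints its type at the stack threshold.
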(event Custom|Friction%20Return
  (Variables|/Script/Engine.CharacterMovementComponent|SetGroundFriction (Variables|Character|GetCharacterMovement) 8.0)
  (Variables|Default|SetKnocking false))

(event Custom|Bleed%20Tick
  (Development|PrintString "Hello")
  (Variables|Default|SetHealth (- (Variables|Default|GetHealth) (* (Variables|Default|GetBleed%20Stacks) 5)))
  (Math|Integer|DecrementInt (Variables|Default|GetBleed%20Ticks%20Left)
    (:%20%20
      (if (<= (Variables|Default|GetBleed%20Ticks%20Left) 0)
        (Utilities|Time|ClearandInvalidateTimerbyHandle (stale EventApplyBleed _returnvalue))
        (Variables|Default|SetBleed%20Stacks 0)
        (Variables|Default|SetBleeding false)
        (elif (<= (Variables|Default|GetHealth) 0.0)
          (bind _player (Class|BPIPlayer|GetPlayer(Message) (Variables|Default|GetBleed%20Player)))
          (Variables|/Game/Blueprints/Player/BP_PlayerCharacter.BP_PlayerCharacter_C|SetPoints _player (+ (Variables|/Game/Blueprints/Player/BP_PlayerCharacter.BP_PlayerCharacter_C|GetPoints _player) 50))
          (Actor|DestroyActor))))))

(event Custom|Acid%20Tick
  (bind _acid_ticks_left (Variables|Default|GetAcid%20Ticks%20Left))
  (Development|PrintString (Utilities|String|ToString(Integer) (Variables|Default|GetAcid%20Stacks)))
  (Variables|Default|SetHealth (- (Variables|Default|GetHealth) (* (Variables|Default|GetAcid%20Stacks) 5)))
  (Math|Integer|DecrementInt _acid_ticks_left
    (:%20%20
      (if (<= _acid_ticks_left 0)
        (Utilities|Time|ClearandInvalidateTimerbyHandle (stale EventApplyAcid _returnvalue))
        (Variables|Default|SetAcid%20Stacks 0)
        (Variables|Default|SetAcid false)
        (elif (<= (Variables|Default|GetHealth) 0.0)
          (bind _player (Class|BPIPlayer|GetPlayer(Message) (Variables|Default|GetAcid%20Player)))
          (Variables|/Game/Blueprints/Player/BP_PlayerCharacter.BP_PlayerCharacter_C|SetPoints _player (+ (Variables|/Game/Blueprints/Player/BP_PlayerCharacter.BP_PlayerCharacter_C|GetPoints _player) 50))
          (Actor|DestroyActor))))))

(event EventBeginPlay
  (bind _self self)
  (AddComponent|AddBPCAssignEnemyStats _self)
  (Variables|Default|SetAIControllerClass "/Script/AIModule.AIController")
  (AI|AIMoveTo _self "0, 0, 0" (Game|GetPlayerCharacter 0) 5.0 false))

(event Collision|EventActorBeginOverlap
  (params (OtherActor :type Actor%20Object%20Reference)))

(event Game|Damage|EventAnyDamage
  (params (Damage :type Float%20%28single-precision%29) (DamageType :type Damage%20Type%20Object%20Reference) (InstigatedBy :type Controller%20Object%20Reference) (DamageCauser :type Actor%20Object%20Reference))
  (Variables|Default|SetHealth (- (Variables|Default|GetHealth) Damage))
  (Utilities|IsValid DamageCauser
    (:Is%20Valid
      (bind _player (Class|BPIPlayer|GetPlayer(Message) DamageCauser))
      (Variables|/Game/Blueprints/Player/BP_PlayerCharacter.BP_PlayerCharacter_C|SetPoints _player (+ (Variables|/Game/Blueprints/Player/BP_PlayerCharacter.BP_PlayerCharacter_C|GetPoints _player) 5))
      (if (<= (Variables|Default|GetHealth) 0.0)
        (bind _player_2 (Class|BPIPlayer|GetPlayer(Message) DamageCauser))
        (Variables|/Game/Blueprints/Player/BP_PlayerCharacter.BP_PlayerCharacter_C|SetPoints _player_2 (+ (Variables|/Game/Blueprints/Player/BP_PlayerCharacter.BP_PlayerCharacter_C|GetPoints _player_2) 50))
        (Actor|DestroyActor)))))

(event EventTick
  (params (DeltaSeconds :type Float%20%28single-precision%29))
  (if (not (Variables|Default|GetKnocking))
    (AI|AIMoveTo self "0, 0, 0" (Game|GetPlayerCharacter 0) 5.0 false)))

(event EventApplyBleed
  (params (Player :type BP%20Player%20Character%20Object%20Reference))
  (if (Variables|Default|GetBleeding)
    (Variables|Default|SetBleed%20Ticks%20Left 16)
    (Math|Integer|IncrementInt (Variables|Default|GetBleed%20Stacks))
    (else
      (bind _returnvalue (Utilities|Time|SetTimerbyEvent (delegate Custom|Bleed%20Tick) 0.25 true))
      (Variables|Default|SetBleed%20Player Player)
      (Variables|Default|SetBleed%20Ticks%20Left 16)
      (Variables|Default|SetBleed%20Stacks 1)
      (Variables|Default|SetBleeding true))))

(event EventKnockback
  (params (Launch%20Velocity :type Vector :default "0, 0, 0"))
  (Variables|Default|SetKnocking true)
  (Components|Movement|StopMovementImmediately (Variables|Character|GetCharacterMovement))
  (Variables|/Script/Engine.CharacterMovementComponent|SetGroundFriction (Variables|Character|GetCharacterMovement) 0.0)
  (Character|LaunchCharacter Launch%20Velocity false false)
  (Utilities|Time|SetTimerbyEvent (delegate Custom|Friction%20Return) 0.3))

(event EventBuildup
  (params (Type :type E_Buildups%20Enum :default "NewEnumerator0") (Player :type BP%20Player%20Character%20Object%20Reference))
  (Math|Integer|IncrementInt (Variables|Default|GetLightning%20Stacks)
    (:%20%20
      (if (>= (Variables|Default|GetLightning%20Stacks) 8)
        (switch Utilities|FlowControl|Switch|SwitchonE_Buildups Type
          (:NewEnumerator0
            (Development|PrintString "Lightning"))
          (:NewEnumerator1
            (Development|PrintString "Chain Lightning"))
          (:NewEnumerator2
            (Development|PrintString "Web Lightning")))
        (Variables|Default|SetLightning%20Stacks 0)))))

(event EventApplyAcid
  (params (Player :type BP%20Player%20Character%20Object%20Reference))
  (if (Variables|Default|GetAcid)
    (Variables|Default|SetAcid%20Ticks%20Left 16)
    (Math|Integer|IncrementInt (Variables|Default|GetAcid%20Stacks))
    (else
      (bind _returnvalue (Utilities|Time|SetTimerbyEvent (delegate Custom|Acid%20Tick) 0.25 true))
      (Variables|Default|SetAcid%20Player Player)
      (Variables|Default|SetAcid%20Ticks%20Left 16)
      (Variables|Default|SetAcid%20Stacks 1)
      (Variables|Default|SetAcid true))))

(fn ConstructionScript)

(fn GetName
  (return "Parent"))