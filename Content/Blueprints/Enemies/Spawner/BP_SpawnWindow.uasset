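; Boarded-up window that spawns BP_Guy1 AI enemies on a looping timer, restarted at a new rate by NewRound, and notifies the level of each spawn.
; Tick checks spawned enemies against PullRange and, after a delay, removes boards while the player isn't building.
; Overlapping the box enables input, letting the player hold Interact to re-add boards in timed stages, with a cooldown after release.
; Windows flagged IsOpen start without boards.
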(event OnComponentBeginOverlap(Box)
  (params (OverlappedComponent :type Primitive%20Component%20Object%20Reference) (OtherActor :type Actor%20Object%20Reference) (OtherComp :type Primitive%20Component%20Object%20Reference) (OtherBodyIndex :type Integer) (bFromSweep :type Boolean) (SweepResult :type Hit%20Result%20Structure%20%28by%20ref%29))
  ;[1 0.9019 0.2125] Toggle Input
  (if (== OtherActor (Game|GetPlayerCharacter 0))
    (Input|EnableInput (Game|GetPlayerController 0))))

(event OnComponentEndOverlap(Box)
  (params (OverlappedComponent :type Primitive%20Component%20Object%20Reference) (OtherActor :type Actor%20Object%20Reference) (OtherComp :type Primitive%20Component%20Object%20Reference) (OtherBodyIndex :type Integer))
  ;[1 0.9019 0.2125] Toggle Input
  (if (== OtherActor (Game|GetPlayerCharacter 0))
    (Input|DisableInput (Game|GetPlayerController 0))))

(event Custom|Spawn
  (bind _actorsfromwindow (Variables|Default|GetactorsFromWindow))
  (Development|PrintString "before branch")
  (if (Variables|Default|GetcanSpawn)
    (Development|PrintString "Spawned")
    (bind _returnvalue (AI|SpawnAIFromClass "/Game/Blueprints/Enemies/Children/BP_Guy1.BP_Guy1_C" 0 (Transformation|GetWorldLocation (Variables|Default|GetArrow)) "0, 0, 0" false 0))
    (Utilities|Array|Add _actorsfromwindow _returnvalue)
    (Variables|Default|SetTotalEnemiesFromWindow (- (Utilities|Array|Length _actorsfromwindow) 1))
    (Class|BPIRoundInteractions|EnemySpawned(Message) (Class|Actor|GetLevel))
    (else
      (Development|PrintString "not spawning"))))

(event Input|EnhancedActionEvents|EnhancedInputActionIA_Interact
  (params (ActionValue :type Boolean) (ElapsedSeconds :type Float%20%28double-precision%29) (TriggeredSeconds :type Float%20%28double-precision%29) (InputAction :type Input%20Action%20Object%20Reference :default "/Game/Blueprints/Game/Input/InputActions/IA_Interact.IA_Interact"))
  (:Triggered
    (if (< ElapsedSeconds 3.2)
      (if (Variables|Default|GetAllowedToBuild)
        (Variables|Default|SetisBuilding true)
        (if (>= ElapsedSeconds 1.0)
          (switch int (Variables|Default|GetCurrentBoards)
            (:Default
              (Development|PrintString (Utilities|String|ToString(Integer) (Variables|Default|GetCurrentBoards)) :!label _label))
            (:0
              (Development|PrintString "1")
              (bind _returnvalue (AddComponent|AddStaticMeshComponent false (Variables|Default|Getboard2Location)))
              (bind _output_get (Variables|Default|SettempBoard _returnvalue))
              (Collision|SetCollisionResponsetoAllChannels _output_get "ECR_Block")
              (Transformation|AttachComponentToComponent _output_get (Variables|Default|GetLeftWindowSill) "None" "KeepRelative" "KeepRelative" "KeepRelative" true)
              (Variables|Default|SetCurrentBoards (+ (Variables|Default|GetCurrentBoards) 1)))
            (:1
              (if (>= ElapsedSeconds 2.0)
                (Development|PrintString "2")
                (bind _returnvalue_2 (AddComponent|AddStaticMeshComponent false (Variables|Default|Getboard1Location)))
                (bind _output_get_2 (Variables|Default|SettempBoard1 _returnvalue_2))
                (Collision|SetCollisionResponsetoAllChannels _output_get_2 "ECR_Block")
                (Transformation|AttachComponentToComponent _output_get_2 (Variables|Default|GetLeftWindowSill) "None" "KeepRelative" "KeepRelative" "KeepRelative" true)
                (Variables|Default|SetCurrentBoards (+ (Variables|Default|GetCurrentBoards) 1))))
            (:2
              (if (>= ElapsedSeconds 3.0)
                (Development|PrintString "3")
                (bind _returnvalue_3 (AddComponent|AddStaticMeshComponent false (Variables|Default|GetboardLocation)))
                (bind _output_get_3 (Variables|Default|SettempBoard2 _returnvalue_3))
                (Collision|SetCollisionResponsetoAllChannels _output_get_3 "ECR_Block")
                (Transformation|AttachComponentToComponent _output_get_3 (Variables|Default|GetLeftWindowSill) "None" "KeepRelative" "KeepRelative" "KeepRelative" true)
                (Variables|Default|SetCurrentBoards (+ (Variables|Default|GetCurrentBoards) 1))))
            (:3
              (goto _label)))))
      (else
        (Variables|Default|SetAllowedToBuild false :!label _label_2)
        (Variables|Default|SetisBuilding false)
        (Utilities|FlowControl|Delay 5.0)
        (Variables|Default|SetAllowedToBuild true))))
  (:Canceled
    (goto _label_2))
  (:Completed
    (goto _label_2)))

(event EventNewRound
  (params (SpawnRate :type Float%20%28double-precision%29))
  (Utilities|Time|ClearandInvalidateTimerbyHandle (stale EventBeginPlay _returnvalue))
  (Utilities|Time|SetTimerbyEvent (delegate Custom|Spawn) SpawnRate true))

(event EventBeginPlay
  (bind _board (Variables|Default|GetBoard))
  (bind _board2 (Variables|Default|GetBoard2))
  (bind _board1 (Variables|Default|GetBoard1))
  ;[0.5677 0.1726 0.04126] Boards Setup
  (if (== (Variables|Default|GetisOpen) true)
    (Components|DestroyComponent _board)
    (Components|DestroyComponent _board1)
    (Components|DestroyComponent _board2)
    (else
      (Variables|Default|SetCurrentBoards 3)
      (Variables|Default|SettempBoard _board)
      (Variables|Default|SettempBoard1 _board1)
      (Variables|Default|SettempBoard2 _board2)))
  (bind _returnvalue (Utilities|Time|SetTimerbyEvent (delegate Custom|Spawn) (Variables|Default|GetspawnRate) true))
  (Development|PrintString "spawn timer started"))

(event EventTick
  (params (DeltaSeconds :type Float%20%28single-precision%29))
  (bind _tempboard (Variables|Default|GettempBoard))
  (bind _tempboard1 (Variables|Default|GettempBoard1))
  (bind _tempboard2 (Variables|Default|GettempBoard2))
  (bind _array_element (Utilities|Array|ForEachLoopwithBreak (Variables|Default|GetactorsFromWindow))
    (:LoopBody
      (Utilities|IsValid _array_element
        (:Is%20Valid
          (if (<= (Math|Vector|Distance2D(Vector) (Math|Conversions|ToVector2D(Vector) (Transformation|GetActorLocation _array_element)) (Math|Conversions|ToVector2D(Vector) (Transformation|GetWorldLocation (Variables|Default|GetPullRange)))) 1e+02)
            (if (not (Variables|Default|GetisBuilding))
              (if (> (Variables|Default|GetCurrentBoards) 0)
                (switch int (Variables|Default|GetCurrentBoards)
                  (:1
                    (Utilities|FlowControl|Delay 1.0)
                    (Utilities|IsValid _tempboard
                      (:Is%20Valid
                        (Components|DestroyComponent _tempboard)
                        (Variables|Default|SetCurrentBoards (- (Variables|Default|GetCurrentBoards) 1)))))
                  (:2
                    (Utilities|FlowControl|Delay 1.0)
                    (Utilities|IsValid _tempboard1
                      (:Is%20Valid
                        (Components|DestroyComponent _tempboard1)
                        (Variables|Default|SetCurrentBoards (- (Variables|Default|GetCurrentBoards) 1)))))
                  (:3
                    (Utilities|FlowControl|Delay 1.0)
                    (Utilities|IsValid _tempboard2
                      (:Is%20Valid
                        (Components|DestroyComponent _tempboard2)
                        (Variables|Default|SetCurrentBoards (- (Variables|Default|GetCurrentBoards) 1))))))))))))))

(fn ConstructionScript)