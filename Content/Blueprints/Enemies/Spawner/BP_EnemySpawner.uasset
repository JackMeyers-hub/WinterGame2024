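; BP_EnemySpawner is a placed actor that keeps spawning AI enemies around itself on a repeating timer.
; BeginPlay starts a looping timer at Interval, and each tick of it spawns a random class from SpawnableEnemies at a random navigable point within Radius.
; The construction script sizes the Sphere component to Radius, so its extent matches the spawn area.
; Spawning has no count limit or stop condition.
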(event Custom|Spawn
  (bind _spawnableenemies (Variables|Default|GetSpawnableEnemies))
  (bind _randomlocation (Class|NavigationSystemV1|GetRandomLocationinNavigableRadius (Transformation|GetActorLocation) (Variables|Default|GetRadius) 0 0))
  (AI|SpawnAIFromClass (Utilities|Array|Get(acopy) _spawnableenemies (Math|Random|RandomInteger (Utilities|Array|Length _spawnableenemies))) 0 _randomlocation "0, 0, 0" false 0))

(event EventBeginPlay
  (Utilities|Time|SetTimerbyEvent (delegate Custom|Spawn) (Variables|Default|GetInterval) true))

(event Collision|EventActorBeginOverlap
  (params (OtherActor :type Actor%20Object%20Reference)))

(event EventTick
  (params (DeltaSeconds :type Float%20%28single-precision%29)))

(fn ConstructionScript
  (Components|Sphere|SetSphereRadius (Variables|Default|GetSphere) (Variables|Default|GetRadius) true))