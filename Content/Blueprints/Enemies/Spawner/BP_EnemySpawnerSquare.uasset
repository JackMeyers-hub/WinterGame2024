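; Enemy spawner that periodically spawns a batch of randomly chosen enemy classes inside a box area, at a rate that ramps up over time.
; Each spawn picks a random point in the box, sized by the Construction Script, and projects it onto the navmesh.
; Tick counts down to lower the spawn interval, then flags the next Spawn to restart its looping timer at the new interval, floored at a minimum.
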(event Custom|Spawn
  (bind _spawnableenemies (Variables|SpawnSettings|GetSpawnableEnemies))
  (for _index (range 0 (- (Variables|SpawnSettings|GetSpawnAmount) 1))
    (AI|SpawnAIFromClass (Utilities|Array|Get(acopy) _spawnableenemies (Math|Random|RandomInteger (Utilities|Array|Length _spawnableenemies))) 0 (.ProjectedLocation (AI|Navigation|ProjectPointtoNavigation (Math|Random|RandomPointinBoundingBox (Transformation|GetActorLocation) (Math|Vector|MakeVector (Variables|SpawnZone|GetLength) (Variables|SpawnZone|GetWidth) (Variables|SpawnZone|GetHeight))) 0 0 (Math|Vector|MakeVector 1e+02 1e+02 (Variables|SpawnZone|GetHeight)))) "0, 0, 0" false 0))
  (if (Variables|Default|GetResetTimer)
    (Variables|Default|SetResetTimer false)
    (Utilities|Time|ClearandInvalidateTimerbyHandle (stale _returnvalue))
    (if (<= (Variables|SpawnSettings|GetSpawn_Interval) (Variables|SpawnSettings|GetSpawnIntervalMin))
      (Utilities|Time|SetTimerbyEvent (delegate Custom|Spawn) (Variables|SpawnSettings|GetSpawnIntervalMin) true)
      (Variables|Default|SetcurrCD (Variables|SpawnSettings|GetDecrease_Interval))
      (else
        (bind _returnvalue (Utilities|Time|SetTimerbyEvent (delegate Custom|Spawn) (Variables|SpawnSettings|GetSpawn_Interval) true))
        (Variables|Default|SetcurrCD (Variables|SpawnSettings|GetDecrease_Interval))))))

(event EventBeginPlay
  (bind _returnvalue (Utilities|Time|SetTimerbyEvent (delegate Custom|Spawn) (Variables|SpawnSettings|GetSpawn_Interval) true))
  (Variables|Default|SetcurrCD (Variables|SpawnSettings|GetDecrease_Interval)))

(event Collision|EventActorBeginOverlap
  (params (OtherActor :type Actor%20Object%20Reference)))

(event EventTick
  (params (DeltaSeconds :type Float%20%28single-precision%29))
  (if (not (Variables|Default|GetResetTimer))
    (Variables|Default|SetcurrCD (- (Variables|Default|GetcurrCD) DeltaSeconds))
    (if (<= (Variables|Default|GetcurrCD) 0.0)
      (Variables|SpawnSettings|SetSpawn_Interval (- (Variables|SpawnSettings|GetSpawn_Interval) (Variables|SpawnSettings|GetDecrease_Amount)))
      (Variables|Default|SetcurrCD (Variables|SpawnSettings|GetDecrease_Interval))
      (Variables|Default|SetResetTimer true))))

(fn ConstructionScript
  (Components|Box|SetBoxExtent (Variables|Default|GetBox) (Math|Vector|MakeVector (Variables|SpawnZone|GetLength) (Variables|SpawnZone|GetWidth) (Variables|SpawnZone|GetHeight)) true))