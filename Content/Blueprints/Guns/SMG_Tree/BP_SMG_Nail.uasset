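; BP_SMG_Nail is a nail projectile from the SMG gun tree that damages and knocks back what it hits.
; On each collision hit it sends a knockback message along its arrow's forward direction and applies damage with the Player as damage causer.
; Each hit also decrements a bounce limit, and the nail destroys itself when that count reaches zero.
; The overlap event is empty, and a duplicate damage-and-bounce chain is left unconnected.
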(event OnComponentHit(Collision)
  (params (HitComponent :type Primitive%20Component%20Object%20Reference) (OtherActor :type Actor%20Object%20Reference) (OtherComp :type Primitive%20Component%20Object%20Reference) (NormalImpulse :type Vector :default "0, 0, 0") (Hit :type Hit%20Result%20Structure%20%28by%20ref%29))
  (Class|BPIEnemies|Knockback(Message) OtherActor (* (Math|Vector|GetForwardVector (Variables|Default|GetArrow)) 6e+02))
  (Game|Damage|ApplyDamage OtherActor (Variables|Default|GetDamage) 0 (Variables|Default|GetPlayer))
  (Math|Integer|DecrementInt (Variables|Default|GetBounce%20Limit)
    (:%20%20
      (if (== (Variables|Default|GetBounce%20Limit) 0)
        (Actor|DestroyActor)))))

(event OnComponentBeginOverlap(Collision)
  (params (OverlappedComponent :type Primitive%20Component%20Object%20Reference) (OtherActor :type Actor%20Object%20Reference) (OtherComp :type Primitive%20Component%20Object%20Reference) (OtherBodyIndex :type Integer) (bFromSweep :type Boolean) (SweepResult :type Hit%20Result%20Structure%20%28by%20ref%29)))

(event EventBeginPlay)

(event Collision|EventActorBeginOverlap
  (params (OtherActor :type Actor%20Object%20Reference)))

(event EventTick
  (params (DeltaSeconds :type Float%20%28single-precision%29)))

(fn ConstructionScript)