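; Lightning chain actor from the SMG gun tree that bounces damage between nearby enemies.
; On Activate it searches all BP_EnemyParent actors once per bounce for the closest within ClosestDistance, excluding only the origin and last-hit enemy.
; It teleports to that target, applies fixed damage credited to Player as causer, and resets the search range.
; It prints each search result for debugging and destroys itself after the loop.
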(event Custom|Activate
  (for _index (range 0 (Variables|Default|GetLightning%20Chain%20Bounces))
    (bind _outactors (Actor|GetAllActorsOfClass "/Game/Blueprints/Enemies/Parent/BP_EnemyParent.BP_EnemyParent_C"))
    (for _array_element _outactors
      (if (and (not (== _array_element (Variables|Default|GetOrigin%20Enemy))) (not (== _array_element (Variables|Default|GetFirst%20Bounced))))
        (if (< (Transformation|GetDistanceTo _array_element) (Variables|Default|GetClosest%20Distance))
          (Variables|Default|SetClosest%20Enemy _array_element)
          (Variables|Default|SetClosest%20Distance (Transformation|GetDistanceTo _array_element)))))
    (Development|PrintString (Utilities|GetDisplayName (Variables|Default|GetClosest%20Enemy)))
    (if (Utilities|IsValid (Variables|Default|GetClosest%20Enemy))
      (Transformation|SetActorLocation (Transformation|GetActorLocation (Variables|Default|GetClosest%20Enemy)) false false)
      (Game|Damage|ApplyDamage (Variables|Default|GetClosest%20Enemy) 1e+02 0 (Variables|Default|GetPlayer))
      (Variables|Default|SetFirst%20Bounced (Variables|Default|GetClosest%20Enemy))
      (Variables|Default|SetClosest%20Enemy 0)
      (Variables|Default|SetClosest%20Distance 5e+02)))
  (Actor|DestroyActor))

(event EventBeginPlay)

(event Collision|EventActorBeginOverlap
  (params (OtherActor :type Actor%20Object%20Reference)))

(event EventTick
  (params (DeltaSeconds :type Float%20%28single-precision%29)))

(fn ConstructionScript)