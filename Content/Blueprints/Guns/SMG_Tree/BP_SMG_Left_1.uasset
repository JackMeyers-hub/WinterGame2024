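; SMG_Left_1 is an SMG gun variant in the weapon upgrade tree that overrides Shoot and passes both upgrade events to its parent.
; When off cooldown, it fires either a hitscan trace with debug drawing or a BP_SMG_Lightning_Bullet projectile, both with random spread.
; Each shot spends ammo, sets the fire-rate cooldown and adds random recoil to the player's Punchangle.
; An empty magazine triggers a reload.
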(event EventBeginPlay
  (|CallParentFunction) ; This node is disabled and will not be called.\nDrag off pins to build functionality.
)

(event Collision|EventActorBeginOverlap
  (params (OtherActor :type Actor%20Object%20Reference))
  (|CallParentFunction OtherActor) ; This node is disabled and will not be called.\nDrag off pins to build functionality.
)

(event EventTick
  (params (DeltaSeconds :type Float%20%28single-precision%29))
  (|CallParentFunction DeltaSeconds) ; This node is disabled and will not be called.\nDrag off pins to build functionality.
)

(event EventShoot
  (params (Damage :type Float%20%28double-precision%29))
  (bind _arrow (Variables|Default|GetArrow))
  (bind _recoil (Variables|Default|GetRecoil))
  (bind _arrow_2 (Variables|Default|GetArrow))
  (bind _spread (Variables|Default|GetSpread))
  (bind _spread_2 (Variables|Default|GetSpread))
  (bind _spread_3 (Variables|Default|GetSpread))
  (bind _spread_4 (Variables|Default|GetSpread))
  (bind _spread_5 (Variables|Default|GetSpread))
  (bind _spread_6 (Variables|Default|GetSpread))
  (bind _returnvalue (Transformation|GetWorldLocation _arrow))
  (bind _returnvalue_2 (Transformation|GetWorldTransform _arrow_2))
  (bind _returnvalue_3 (* _spread_2 -1.0))
  (bind _returnvalue_4 (* _spread_4 -1.0))
  (bind _returnvalue_5 (* _spread_6 -1.0))
  (bind _returnvalue_6 (Math|Random|RandomFloatinRange _returnvalue_4 _spread_3))
  (bind _returnvalue_7 (Math|Random|RandomFloatinRange _returnvalue_5 _spread_5))
  (bind _returnvalue_8 (Math|Random|RandomFloatinRange _returnvalue_3 _spread))
  (bind _returnvalue_9 (/ _returnvalue_8 3.0))
  (bind _returnvalue_10 (/ _returnvalue_6 3.0))
  (bind _returnvalue_11 (/ _returnvalue_7 3.0))
  ;[1 0.2682 0.3279] Shoot
  (if (<= (Variables|Default|GetShootCD) 0.0)
    (if (> (Variables|Default|GetCurrMagAmmo) 0)
      (if (Variables|Default|GetIsHitscan)
        (Utilities|FlowControl|Sequence
          (:then_0
            (bind _outhit (Collision|LineTraceByChannel _returnvalue (+ _returnvalue (* (Math|Vector|RotateVector (Math|Vector|GetForwardVector _arrow) (Math|Rotator|MakeRotator _returnvalue_9 _returnvalue_10 _returnvalue_11)) 1e+05)) "TraceTypeQuery1" false 0 "ForDuration"))
            (Game|Damage|ApplyDamage (.hitactor _outhit) (Variables|Default|GetDamage) 0 (Variables|Default|GetPlayer)))
          (:then_1
            (Variables|Default|SetCurrMagAmmo (- (Variables|Default|GetCurrMagAmmo) 1) :!label _label)
            (Variables|Default|SetShootCD (/ 1.0 (Variables|Default|GetFirerate)))
            (bind _player (Class|BPIPlayer|GetPlayer(Message) (Game|GetPlayerCharacter 0)))
            (Variables|/Game/Blueprints/Player/BP_PlayerCharacter.BP_PlayerCharacter_C|SetPunchangle _player (Math|Rotator|MakeRotator (+ (.roll (Variables|/Game/Blueprints/Player/BP_PlayerCharacter.BP_PlayerCharacter_C|GetPunchangle _player)) (Math|Random|RandomFloatinRange (* _recoil -1.0) _recoil)) (+ (.pitch (Variables|/Game/Blueprints/Player/BP_PlayerCharacter.BP_PlayerCharacter_C|GetPunchangle _player)) (Math|Random|RandomFloatinRange (* _recoil 0.5) (* _recoil 2.0))) (+ (.yaw (Variables|/Game/Blueprints/Player/BP_PlayerCharacter.BP_PlayerCharacter_C|GetPunchangle _player)) 0.0)))))
        (else
          (Utilities|FlowControl|Sequence
            (:then_0
              (bind _returnvalue_12 (Game|SpawnActorfromClass "/Game/Blueprints/Guns/SMG_Tree/BP_SMG_Lightning_Bullet.BP_SMG_Lightning_Bullet_C" (Math|Transform|MakeTransform (.location _returnvalue_2) (Math|Rotator|MakeRotator (+ (.roll (.rotation _returnvalue_2)) _returnvalue_9) (+ (.pitch (.rotation _returnvalue_2)) _returnvalue_10) (+ (.yaw (.rotation _returnvalue_2)) _returnvalue_11)) "1.000000,1.000000,1.000000") "AdjustIfPossibleButAlwaysSpawn" "MultiplyWithRoot" 0 0))
              (if (Utilities|IsValid _returnvalue_12)
                (Variables|/Game/Blueprints/Guns/SMG_Tree/BP_SMG_Lightning_Bullet.BP_SMG_Lightning_Bullet_C|SetDamage _returnvalue_12 Damage)
                (Variables|/Game/Blueprints/Guns/SMG_Tree/BP_SMG_Lightning_Bullet.BP_SMG_Lightning_Bullet_C|SetPlayer _returnvalue_12 (Variables|Default|GetPlayer))
                (Variables|/Game/Blueprints/Guns/SMG_Tree/BP_SMG_Lightning_Bullet.BP_SMG_Lightning_Bullet_C|SetType _returnvalue_12 "NewEnumerator0")))
            (:then_1
              (goto _label)))))
      (else
        (CallFunction|Reload)))))

(event EventUpgradeLeft
  (|CallParentFunction))

(event EventUpgradeRight
  (|CallParentFunction))

(fn ConstructionScript
  (|CallParentFunction))

(fn GetName
  (return "SMG_Left_1"))