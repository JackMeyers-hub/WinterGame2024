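; Web lightning effect from the SMG tree that, on Activate, deals flat damage to up to three enemies near an origin enemy.
; It scans all BP_EnemyParent actors within Range, skipping OriginEnemy, and fills three target slots.
; Once full, closer candidates replace the tracked furthest target and become the new furthest without rechecking the others, so the result is not guaranteed nearest.
; Damage is credited to Player as causer.
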(event Custom|Activate
  (bind _returnvalue (Transformation|GetDistanceTo 0))
  (bind _player (Variables|Default|GetPlayer))
  (bind _outactors (Actor|GetAllActorsOfClass "/Game/Blueprints/Enemies/Parent/BP_EnemyParent.BP_EnemyParent_C"))
  (for _array_element _outactors
    (if (not (== _array_element (Variables|Default|GetOrigin%20Enemy)))
      (if (<= _returnvalue (Variables|Default|GetRange))
        (if (Variables|Default|GetFilled%20Targets)
          (if (< _returnvalue (Variables|Default|GetFurthestDistance))
            (Utilities|FlowControl|Sequence
              (:then_0
                (if (== (Variables|Default|GetFurtherstEnemy) (Variables|Default|GetTarget1))
                  (Variables|Default|SetTarget1 _array_element)
                  (Variables|Default|SetFurtherstEnemy _array_element :!label _label)
                  (Variables|Default|SetFurthestDistance (Transformation|GetDistanceTo _array_element))))
              (:then_1
                (if (== (Variables|Default|GetFurtherstEnemy) (Variables|Default|GetTarget2))
                  (Variables|Default|SetTarget2 _array_element)
                  (goto _label)))
              (:then_2
                (if (== (Variables|Default|GetFurtherstEnemy) (Variables|Default|GetTarget3))
                  (Variables|Default|SetTarget3 _array_element)
                  (goto _label)))))
          (else
            (Variables|Default|SetTarget3 (Variables|Default|GetTarget2))
            (Variables|Default|SetTarget2 (Variables|Default|GetTarget1))
            (Variables|Default|SetTarget1 _array_element)
            (Utilities|FlowControl|Sequence
              (:then_0
                (if (> (Transformation|GetDistanceTo _array_element) (Variables|Default|GetFurthestDistance))
                  (Variables|Default|SetFurthestDistance (Transformation|GetDistanceTo _array_element))
                  (Variables|Default|SetFurtherstEnemy _array_element)))
              (:then_1
                (if (not (== (Variables|Default|GetTarget3) 0))
                  (Variables|Default|SetFilled%20Targets true)))))))))
  (Game|Damage|ApplyDamage (Variables|Default|GetTarget1) 5e+01 0 _player)
  (Game|Damage|ApplyDamage (Variables|Default|GetTarget2) 5e+01 0 _player)
  (Game|Damage|ApplyDamage (Variables|Default|GetTarget3) 5e+01 0 _player))

(event EventBeginPlay)

(event Collision|EventActorBeginOverlap
  (params (OtherActor :type Actor%20Object%20Reference)))

(event EventTick
  (params (DeltaSeconds :type Float%20%28single-precision%29)))

(fn ConstructionScript)