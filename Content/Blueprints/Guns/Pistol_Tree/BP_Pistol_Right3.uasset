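; BP_Pistol_Right3 is a gun Blueprint in the pistol upgrade tree, named as the third step on the right branch.
; BeginPlay, overlap, Tick, Shoot and both upgrade events only forward to the parent class, so all behavior is inherited.
; Its only logic of its own is GetName, which returns a hardcoded identifier for this variant.
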(event EventBeginPlay
  (|CallParentFunction))

(event Collision|EventActorBeginOverlap
  (params (OtherActor :type Actor%20Object%20Reference))
  (|CallParentFunction OtherActor))

(event EventTick
  (params (DeltaSeconds :type Float%20%28single-precision%29))
  (|CallParentFunction DeltaSeconds))

(event EventShoot
  (params (Damage :type Float%20%28double-precision%29))
  (|CallParentFunction Damage))

(event EventUpgradeLeft
  (|CallParentFunction))

(event EventUpgradeRight
  (|CallParentFunction))

(fn ConstructionScript)

(fn GetName
  (return "Pistol_Right_3"))