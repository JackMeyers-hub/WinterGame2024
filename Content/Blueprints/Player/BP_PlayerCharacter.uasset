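; Player character that handles movement, look, jump and a two-slot weapon inventory with pickup, swap, fire and reload.
; Weapons attach to arrow components for equipped and secondary slots, and pickup with both full drops the equipped one with physics.
; Input fires once on press, repeating only for automatic weapons.
; RepNotify variables update HUD ammo and points, the weapon's owner and camera recoil, which a looping timer decays.
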(event Custom|RecoilReset
  (Variables|Default|SetPunchangle (* (Variables|Default|GetPunchangle) 0.95)))

(event Input|EnhancedActionEvents|EnhancedInputActionIA_Move
  (params (ActionValue :type Vector%202D%20Structure) (ElapsedSeconds :type Float%20%28double-precision%29) (TriggeredSeconds :type Float%20%28double-precision%29) (InputAction :type Input%20Action%20Object%20Reference :default "/Game/Blueprints/Game/Input/InputActions/IA_Move.IA_Move"))
  (Pawn|Input|AddMovementInput (Transformation|GetActorRightVector) (.x ActionValue) false)
  (Pawn|Input|AddMovementInput (Transformation|GetActorForwardVector) (.y ActionValue) false))

(event Input|EnhancedActionEvents|EnhancedInputActionIA_Camera
  (params (ActionValue :type Vector%202D%20Structure) (ElapsedSeconds :type Float%20%28double-precision%29) (TriggeredSeconds :type Float%20%28double-precision%29) (InputAction :type Input%20Action%20Object%20Reference :default "/Game/Blueprints/Game/Input/InputActions/IA_Camera.IA_Camera"))
  (Pawn|Input|AddControllerYawInput (.x ActionValue))
  (Pawn|Input|AddControllerPitchInput (* (.y ActionValue) -1.0)))

(event Input|EnhancedActionEvents|EnhancedInputActionIA_Shoot
  (params (ActionValue :type Boolean) (ElapsedSeconds :type Float%20%28double-precision%29) (TriggeredSeconds :type Float%20%28double-precision%29) (InputAction :type Input%20Action%20Object%20Reference :default "/Game/Blueprints/Game/Input/InputActions/IA_Shoot.IA_Shoot"))
  (bind _equiped_weapon (Variables|Default|GetEquiped%20Weapon))
  (:Triggered
    (if (Utilities|IsValid _equiped_weapon) :!label _label
      (if (Variables|/Game/Blueprints/Guns/BP_GunParent.BP_GunParent_C|GetIsAutomatic _equiped_weapon)
        (Class|BPIGuns|Shoot(Message) _equiped_weapon (Variables|/Game/Blueprints/Guns/BP_GunParent.BP_GunParent_C|GetDamage _equiped_weapon) :!label _label_2))))
  (:Started
    (goto _label_2))
  (:Ongoing
    (goto _label)))

(event Input|EnhancedActionEvents|EnhancedInputActionIA_Pickup
  (params (ActionValue :type Boolean) (ElapsedSeconds :type Float%20%28double-precision%29) (TriggeredSeconds :type Float%20%28double-precision%29) (InputAction :type Input%20Action%20Object%20Reference :default "/Game/Blueprints/Game/Input/InputActions/IA_Pickup.IA_Pickup"))
  (CallFunction|PickUpWeapons))

(event Input|EnhancedActionEvents|EnhancedInputActionIA_Jump
  (params (ActionValue :type Boolean) (ElapsedSeconds :type Float%20%28double-precision%29) (TriggeredSeconds :type Float%20%28double-precision%29) (InputAction :type Input%20Action%20Object%20Reference :default "/Game/Blueprints/Game/Input/InputActions/IA_Jump.IA_Jump"))
  (Character|Jump))

(event Input|EnhancedActionEvents|EnhancedInputActionIA_SwapWeapons
  (params (ActionValue :type Boolean) (ElapsedSeconds :type Float%20%28double-precision%29) (TriggeredSeconds :type Float%20%28double-precision%29) (InputAction :type Input%20Action%20Object%20Reference :default "/Game/Blueprints/Game/Input/InputActions/IA_SwapWeapons.IA_SwapWeapons"))
  (CallFunction|SwapWeapons))

(event Input|EnhancedActionEvents|EnhancedInputActionIA_Reload
  (params (ActionValue :type Boolean) (ElapsedSeconds :type Float%20%28double-precision%29) (TriggeredSeconds :type Float%20%28double-precision%29) (InputAction :type Input%20Action%20Object%20Reference :default "/Game/Blueprints/Game/Input/InputActions/IA_Reload.IA_Reload"))
  (Class|BPIGuns|Reload(Message) (Variables|Default|GetEquiped%20Weapon)))

(event EventBeginPlay
  (Utilities|Time|SetTimerbyEvent (delegate Custom|RecoilReset) 0.01 true)
  (bind _returnvalue (UserInterface|CreateWidget "/Game/Blueprints/UI/WBP_Hud.WBP_Hud_C"))
  (UserInterface|Viewport|AddtoViewport _returnvalue 0)
  (Variables|Default|SetHud _returnvalue))

(event Collision|EventActorBeginOverlap
  (params (OtherActor :type Actor%20Object%20Reference)))

(event EventTick
  (params (DeltaSeconds :type Float%20%28single-precision%29)))

(event EventSetGroundWeapon
  (params (Weapon :type BP%20Gun%20Parent%20Object%20Reference))
  (Variables|Default|SetGround%20Weapon Weapon))

(fn ConstructionScript)

(fn PickUpWeapons
  (if (!= (Variables|Default|GetGround%20Weapon) 0)
    (if (== (Variables|Default|GetEquiped%20Weapon) 0)
      (Physics|SetSimulatePhysics (Variables|/Game/Blueprints/Guns/BP_GunParent.BP_GunParent_C|GetBody (Variables|Default|GetGround%20Weapon)) false)
      (Transformation|AttachComponentToComponent (Variables|Default|GetGround%20Weapon) (Variables|Default|GetArrow1) "None" "SnapToTarget" "SnapToTarget" "KeepRelative" true)
      (Variables|Default|SetEquiped%20Weapon (Variables|Default|GetGround%20Weapon))
      (Variables|Default|SetGround%20Weapon 0)
      (elif (== (Variables|Default|GetSecondary%20Weapon) 0)
        (Transformation|DetachFromActor (Variables|Default|GetEquiped%20Weapon) "KeepWorld" "KeepWorld" "KeepWorld")
        (Transformation|AttachComponentToComponent (Variables|Default|GetEquiped%20Weapon) (Variables|Default|GetArrow2) "None" "SnapToTarget" "SnapToTarget" "KeepRelative" true)
        (Variables|Default|SetSecondary%20Weapon (Variables|Default|GetEquiped%20Weapon))
        (Variables|Default|SetEquiped%20Weapon 0)
        (Physics|SetSimulatePhysics (Variables|/Game/Blueprints/Guns/BP_GunParent.BP_GunParent_C|GetBody (Variables|Default|GetGround%20Weapon)) false)
        (Transformation|AttachComponentToComponent (Variables|Default|GetGround%20Weapon) (Variables|Default|GetArrow1) "None" "SnapToTarget" "SnapToTarget" "KeepRelative" true)
        (Variables|Default|SetEquiped%20Weapon (Variables|Default|GetGround%20Weapon))
        (else
          (Transformation|DetachFromActor (Variables|Default|GetEquiped%20Weapon) "KeepWorld" "KeepWorld" "KeepWorld")
          (Physics|SetSimulatePhysics (Variables|/Game/Blueprints/Guns/BP_GunParent.BP_GunParent_C|GetBody (Variables|Default|GetEquiped%20Weapon)) true)
          (Variables|Default|SetEquiped%20Weapon 0)
          (Physics|SetSimulatePhysics (Variables|/Game/Blueprints/Guns/BP_GunParent.BP_GunParent_C|GetBody (Variables|Default|GetGround%20Weapon)) false)
          (Transformation|AttachComponentToComponent (Variables|Default|GetGround%20Weapon) (Variables|Default|GetArrow1) "None" "SnapToTarget" "SnapToTarget" "KeepRelative" true)
          (Variables|Default|SetEquiped%20Weapon (Variables|Default|GetGround%20Weapon))
          (Variables|Default|SetGround%20Weapon 0))))))

(fn SwapWeapons
  (if (and (!= (Variables|Default|GetEquiped%20Weapon) 0) (!= (Variables|Default|GetSecondary%20Weapon) 0))
    (Transformation|DetachFromActor (Variables|Default|GetEquiped%20Weapon) "KeepWorld" "KeepWorld" "KeepWorld")
    (Transformation|DetachFromActor (Variables|Default|GetSecondary%20Weapon) "KeepWorld" "KeepWorld" "KeepWorld")
    (Transformation|AttachComponentToComponent (Variables|Default|GetEquiped%20Weapon) (Variables|Default|GetArrow2) "None" "SnapToTarget" "SnapToTarget" "KeepRelative" true)
    (Transformation|AttachComponentToComponent (Variables|Default|GetSecondary%20Weapon) (Variables|Default|GetArrow1) "None" "SnapToTarget" "SnapToTarget" "KeepRelative" true)
    (Variables|Default|SetTempWeapon (Variables|Default|GetSecondary%20Weapon))
    (Variables|Default|SetSecondary%20Weapon (Variables|Default|GetEquiped%20Weapon))
    (Variables|Default|SetEquiped%20Weapon (Variables|Default|GetTempWeapon))
    (Variables|Default|SetTempWeapon 0)))

(fn OnRepPunchangle
  (Transformation|SetRelativeRotation (Variables|Default|GetCamera) (Variables|Default|GetPunchangle) false false))

(fn OnRepEquipedWeapon
  (bind _hud (Variables|Default|GetHud))
  (bind _equiped_weapon (Variables|Default|GetEquiped%20Weapon))
  (if (Utilities|IsValid _equiped_weapon)
    (Variables|/Game/Blueprints/UI/WBP_Hud.WBP_Hud_C|SetCurrMagAmmo _hud (Variables|/Game/Blueprints/Guns/BP_GunParent.BP_GunParent_C|GetCurrMagAmmo _equiped_weapon))
    (Variables|/Game/Blueprints/UI/WBP_Hud.WBP_Hud_C|SetCurrAmmo _hud (Variables|/Game/Blueprints/Guns/BP_GunParent.BP_GunParent_C|GetCurrAmmo _equiped_weapon))
    (Variables|/Game/Blueprints/Guns/BP_GunParent.BP_GunParent_C|SetPlayer _equiped_weapon self)))

(fn OnRepPoints
  (Variables|/Game/Blueprints/UI/WBP_Hud.WBP_Hud_C|SetPointValue (Variables|Default|GetHud) (Variables|Default|GetPoints)))

(fn GetPlayer
  (return self))