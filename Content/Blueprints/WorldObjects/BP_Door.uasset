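; BP_Door is a points-locked door that the player pays to remove.
; When the player character overlaps its Box with more points than PointsToUnlock, the door enables input, then disables it when they leave.
; Triggering IA_Interact deducts the cost from the overlapping actor and destroys the door.
; Points are read and removed through message calls on that actor, with no cast to a player class.
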(event OnComponentBeginOverlap(Box)
  (params (OverlappedComponent :type Primitive%20Component%20Object%20Reference) (OtherActor :type Actor%20Object%20Reference) (OtherComp :type Primitive%20Component%20Object%20Reference) (OtherBodyIndex :type Integer) (bFromSweep :type Boolean) (SweepResult :type Hit%20Result%20Structure%20%28by%20ref%29))
  ;[1 1 1] Comment
  (bind _player (Class|BPIPlayer|GetPlayer(Message) OtherActor))
  (Utilities|IsValid _player
    (:Is%20Valid
      (if (> (Variables|/Game/Blueprints/Player/BP_PlayerCharacter.BP_PlayerCharacter_C|GetPoints _player) (Variables|Default|GetpointsToUnlock))
        (if (== OtherActor (Game|GetPlayerCharacter 0))
          (Input|EnableInput (Game|GetPlayerController 0)))))))

(event OnComponentEndOverlap(Box)
  (params (OverlappedComponent :type Primitive%20Component%20Object%20Reference) (OtherActor :type Actor%20Object%20Reference) (OtherComp :type Primitive%20Component%20Object%20Reference) (OtherBodyIndex :type Integer))
  ;[1 1 1] Comment
  (if (== OtherActor (Game|GetPlayerCharacter 0))
    (Input|DisableInput (Game|GetPlayerController 0))))

(event Input|EnhancedActionEvents|EnhancedInputActionIA_Interact
  (params (ActionValue :type Boolean) (ElapsedSeconds :type Float%20%28double-precision%29) (TriggeredSeconds :type Float%20%28double-precision%29) (InputAction :type Input%20Action%20Object%20Reference :default "/Game/Blueprints/Game/Input/InputActions/IA_Interact.IA_Interact"))
  (:Triggered
    (Class|BPIPlayer|RemovePoints(Message) (stale OnComponentBeginOverlap(Box) OtherActor) (Variables|Default|GetpointsToUnlock))
    (Actor|DestroyActor)))

(event EventBeginPlay)

(event Collision|EventActorBeginOverlap
  (params (OtherActor :type Actor%20Object%20Reference)))

(event EventTick
  (params (DeltaSeconds :type Float%20%28single-precision%29)))

(fn ConstructionScript)

(fn GetPlayer
  (return 0))