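; BP_PointsBank is a world object that holds a points total and shows how full it is through the height of its Bloob component.
; When Points replicates, OnRep_Points sets Bloob's relative Z from the ratio of Points to CurrentPointCap, rounded into discrete steps, leaving X and Y unchanged.
; Tick copies Points into PrevPoints, which nothing else in these graphs reads.
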(event EventBeginPlay)

(event Collision|EventActorBeginOverlap
  (params (OtherActor :type Actor%20Object%20Reference)))

(event EventTick
  (params (DeltaSeconds :type Float%20%28single-precision%29))
  (Variables|Default|SetprevPoints (Variables|Default|GetPoints)))

(fn ConstructionScript)

(fn OnRepPoints
  (bind _bloob (Variables|Default|Getbloob))
  (bind _relativelocation (Variables|/Script/Engine.SceneComponent|GetRelativeLocation _bloob))
  (Transformation|SetRelativeLocation _bloob (Math|Vector|MakeVector (.x _relativelocation) (.y _relativelocation) (Math|Conversions|ToFloat(Integer) (* (Math|Float|Round (* (/ (Variables|Default|GetPoints) (Variables|Default|GetCurrentPointCap)) 1e+01)) 10))) false false))