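; Upgrade station world object that lets the player apply a right or left upgrade to the equipped weapon.
; A hit on the right or left board selects the pending upgrade.
; The box trigger toggles input for the player, so Interact works inside it.
; Interact fetches the equipped weapon through a player message call, checks that side's upgrade state, sends the matching upgrade message and clears the selection.
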(event OnComponentBeginOverlap(Box)
  (params (OverlappedComponent :type Primitive%20Component%20Object%20Reference) (OtherActor :type Actor%20Object%20Reference) (OtherComp :type Primitive%20Component%20Object%20Reference) (OtherBodyIndex :type Integer) (bFromSweep :type Boolean) (SweepResult :type Hit%20Result%20Structure%20%28by%20ref%29))
  ;[1 0.9019 0.2125] Toggle Input
  (if (== OtherActor (Game|GetPlayerCharacter 0))
    (Input|EnableInput (Game|GetPlayerController 0))))

(event OnComponentEndOverlap(Box)
  (params (OverlappedComponent :type Primitive%20Component%20Object%20Reference) (OtherActor :type Actor%20Object%20Reference) (OtherComp :type Primitive%20Component%20Object%20Reference) (OtherBodyIndex :type Integer))
  ;[1 0.9019 0.2125] Toggle Input
  (if (== OtherActor (Game|GetPlayerCharacter 0))
    (Input|DisableInput (Game|GetPlayerController 0))))

(event OnComponentHit(LeftBoard)
  (params (HitComponent :type Primitive%20Component%20Object%20Reference) (OtherActor :type Actor%20Object%20Reference) (OtherComp :type Primitive%20Component%20Object%20Reference) (NormalImpulse :type Vector :default "0, 0, 0") (Hit :type Hit%20Result%20Structure%20%28by%20ref%29))
  ;[1 0.9511 0.295] Sets which upgrade will happen
  (Variables|Default|SetUpgrade 2))

(event OnComponentHit(RightBoard)
  (params (HitComponent :type Primitive%20Component%20Object%20Reference) (OtherActor :type Actor%20Object%20Reference) (OtherComp :type Primitive%20Component%20Object%20Reference) (NormalImpulse :type Vector :default "0, 0, 0") (Hit :type Hit%20Result%20Structure%20%28by%20ref%29))
  ;[1 0.9511 0.295] Sets which upgrade will happen
  (Variables|Default|SetUpgrade 1))

(event Input|EnhancedActionEvents|EnhancedInputActionIA_Interact
  (params (ActionValue :type Boolean) (ElapsedSeconds :type Float%20%28double-precision%29) (TriggeredSeconds :type Float%20%28double-precision%29) (InputAction :type Input%20Action%20Object%20Reference :default "/Game/Blueprints/Game/Input/InputActions/IA_Interact.IA_Interact"))
  (bind _returnvalue (Game|GetPlayerCharacter 0))
  ;[0.4025 1 0.3379] Upgrades Equiped Weapon
  (if (Collision|IsOverlappingActor (Variables|Default|GetBox) _returnvalue :!class /Script/Engine.PrimitiveComponent)
    (bind _player (Class|BPIPlayer|GetPlayer(Message) _returnvalue))
    (switch int (Variables|Default|GetUpgrade)
      (:1
        (if (not (== (Variables|/Game/Blueprints/Guns/BP_GunParent.BP_GunParent_C|GetRight_Upgrade (Variables|/Game/Blueprints/Player/BP_PlayerCharacter.BP_PlayerCharacter_C|GetEquiped%20Weapon _player)) 0))
          (Class|BPIGuns|UpgradeRight(Message) (Variables|/Game/Blueprints/Player/BP_PlayerCharacter.BP_PlayerCharacter_C|GetEquiped%20Weapon _player))
          (Variables|Default|SetUpgrade 0 :!label _label)))
      (:2
        (if (not (== (Variables|/Game/Blueprints/Guns/BP_GunParent.BP_GunParent_C|GetLeft_Upgrade (Variables|/Game/Blueprints/Player/BP_PlayerCharacter.BP_PlayerCharacter_C|GetEquiped%20Weapon _player)) 0))
          (Class|BPIGuns|UpgradeLeft(Message) (Variables|/Game/Blueprints/Player/BP_PlayerCharacter.BP_PlayerCharacter_C|GetEquiped%20Weapon _player))
          (goto _label))))))

(event EventBeginPlay)

(event Collision|EventActorBeginOverlap
  (params (OtherActor :type Actor%20Object%20Reference)))

(event EventTick
  (params (DeltaSeconds :type Float%20%28single-precision%29)))

(fn ConstructionScript)